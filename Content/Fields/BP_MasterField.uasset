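; BP_MasterField is a temporary field actor that passes its charges to receivers entering it.
; On begin overlap it calls AddStack for each FieldCharge entry on an EssentialMatter or EssentialEntity flagged IsReceiver, with a debug print for entities.
; Tick subtracts a fixed step from FieldLifespan, so lifetime depends on frame rate, and destroys the actor at zero.
; The IsStable check on Tick has no effect.
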(event EventBeginPlay)

(event Collision|EventActorBeginOverlap
  (params (OtherActor :type Actor%20Object%20Reference))
  (bind _asbp_essential_matter (Utilities|Casting|CastToBP_EssentialMatter OtherActor)
    (:then
      (if (Variables|/Game/TestEquipment/Objects/BP_EssentialMatter.BP_EssentialMatter_C|GetisReceiver _asbp_essential_matter)
        (for _array_element (Variables|Default|GetFieldCharge)
          (Default|AddStack _asbp_essential_matter _array_element))))
    (:CastFailed
      (bind _asbp_essential_entity (Utilities|Casting|CastToBP_EssentialEntity OtherActor))
      (Development|PrintString "FieldtoChar")
      (if (Variables|/Game/TestEquipment/Characters/BP_EssentialEntity.BP_EssentialEntity_C|GetisReceiver _asbp_essential_entity)
        (for _array_element_2 (Variables|Default|GetFieldCharge)
          (Default|AddStack _asbp_essential_entity _array_element_2))))))

(event EventTick
  (params (DeltaSeconds :type Float%20%28single-precision%29))
  (if (Variables|Default|GetisStable)
    _
    (else
      _))
  (bind _output_get (Variables|Default|SetFieldLifespan (- (Variables|Default|GetFieldLifespan) 0.1)))
  (if (<= _output_get 0.0)
    (Actor|DestroyActor)))

(fn ConstructionScript)